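; Base swivel cannon structure for ship combat that seats a rider standing behind or beside it, offset along its forward axis.
; Placement sphere-traces check tilt, obstruction, ground distance and standing room, mapping failures to custom reason strings.
; Rider position comes from a socket or ground trace, with a delayed client-side re-snap if too far.
; Also overrides the seated camera and plays a Greek fire start sound.
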(fn ConstructionScript)

(fn GetFixedRiderLocation
  (bind _skeletalmesh1 (Variables|Default|GetSkeletalMesh1))
  (bind _ridersocketname (Variables|Default|GetRiderSocketName))
  (bind _returnvalue (Transformation|GetSocketTransform _skeletalmesh1 _ridersocketname "RTS_World"))
  (bind (_location _rotation) (Math|Transform|BreakTransform _returnvalue))
  (Utilities|FlowControl|Sequence
    (:then_0
      (if (not (Variables|Default|GetbSnappedIgnoreGroundForStandingLocation))
        (bind (_loc _rot) (CallFunction|GetStandingLocationRotation (Variables|Default|GetTraceType)))
        (LocalVariables|SetTheLoc _loc)
        (LocalVariables|SetTheRot _rot)
        (if (not (Networking|IsDedicatedServer))
          (Utilities|IsValid (Variables|Default|GetSeatedCharacter)
            (:Is%20Valid
              (if (not (Variables|Default|GetbFirstTimeToSetStanding))
                (Variables|Default|SetbFirstTimeToSetStanding true)
                (bind _bisvalid (CallFunction|IsLocCloseEnough _loc))
                (if (not _bisvalid)
                  (Utilities|Time|SetTimerbyFunctionName self "LookForStandingLocation" (Math|Random|RandomFloatinRange 3.0 5.0)))))))
        (else
          (Class|SkeletalMeshComponent|AbsoluteForceRefreshPoseandTransforms _skeletalmesh1)
          (LocalVariables|SetTheLoc _location)
          (LocalVariables|SetTheRot _rotation))))
    (:then_1
      (return (LocalVariables|GetTheLoc) (LocalVariables|GetTheRot)))))

(fn BPIsAllowedtoBuild
  (params (OutPlacementData :type Placement%20Data%20Structure%20%28by%20ref%29) (CurrentAllowedReason :type Integer))
  (bind (_adjustedlocation _adjustedrotation _bsnapped _bdisableencroachmentcheck _biswatergrounded _mysnaptoindex _theirsnaptoindex _floorhitactor) (Utilities|Struct|BreakPlacementData OutPlacementData))
  (bind _returnvalue (Math|Vector|MakeVector 0.0 0.0 4e+01))
  (bind _rideroffset (Variables|Default|GetRiderOffset))
  (bind _returnvalue_2 (Math|Vector|GetForwardVector _adjustedrotation))
  (bind _returnvalue_3 (Math|Vector|RotateVector _returnvalue _adjustedrotation))
  (bind (_pitch _yaw _roll) (Class|KismetMathLibrary|BreakRot _adjustedrotation))
  (bind _returnvalue_4 (* _returnvalue_2 _rideroffset))
  (bind _returnvalue_5 (+ _adjustedlocation _returnvalue_3))
  (bind _returnvalue_6 (+ _returnvalue_5 _returnvalue_4))
  (bind (_x _y _z) (Math|Vector|BreakVector _returnvalue_6))
  (bind (_x_2 _y_2 _z_2) (Math|Vector|BreakVector _returnvalue_6))
  (LocalVariables|SetCurrentReason CurrentAllowedReason)
  (Utilities|FlowControl|Sequence
    (:then_0
      (if (not _bsnapped)
        (Utilities|Casting|CastToPrimalStructure _floorhitactor
          (:then
            (Utilities|FlowControl|Sequence
              (:then_0
                (if (or (> (Math|Float|Absolute(Float) _pitch) (Variables|Default|GetMaxPlacementPitch)) (> (Math|Float|Absolute(Float) _roll) (Variables|Default|GetMaxPlacementRoll)))
                  (LocalVariables|SetCurrentReason -979)))
              (:then_1
                (bind _returnvalue_7 (Class|KismetSystemLibrary|SphereTraceSingleNEW _returnvalue_5 _returnvalue_6 5.0 (Variables|Default|GetTraceType) false 0 "None" true))
                (if _returnvalue_7
                  (LocalVariables|SetCurrentReason -978)
                  (else
                    (bind _returnvalue_8 (Class|KismetSystemLibrary|SphereTraceSingleNEW _returnvalue_6 (Math|Vector|MakeVector _x _y (- _z (Variables|Default|GetMinDistanceFromGround))) 2e+01 (Variables|Default|GetTraceType) false 0 "None" true))
                    (if _returnvalue_8
                      (LocalVariables|SetCurrentReason -975)
                      (else
                        (bind (_outhit _returnvalue_9) (Class|KismetSystemLibrary|SphereTraceSingleNEW _returnvalue_6 (Math|Vector|MakeVector _x_2 _y_2 (- _z_2 (Variables|Default|GetLookForGroundDistance))) 2e+01 (Variables|Default|GetTraceType) false 0 "None" true))
                        (if _returnvalue_9
                          (bind _returnvalue_10 (Class|KismetSystemLibrary|SphereTraceSingleNEW (.Location (Collision|BreakHitResult _outhit)) (Math|Vector|MakeVector (.X (Math|Vector|BreakVector (.Location (Collision|BreakHitResult _outhit)))) (.Y (Math|Vector|BreakVector (.Location (Collision|BreakHitResult _outhit)))) (+ (.Z (Math|Vector|BreakVector (.Location (Collision|BreakHitResult _outhit)))) (* 86.0 2.0))) 2e+01 (Variables|Default|GetTraceType) false (Utilities|Array|MakeArray (.HitActor (Collision|BreakHitResult _outhit))) "None" true))
                          (if _returnvalue_10
                            (LocalVariables|SetCurrentReason -976)
                            (else
                              (bind _returnvalue_11 (CallFunction|BPAllowSeating))
                              (if (not _returnvalue_11)
                                (LocalVariables|SetCurrentReason -974))))
                          (else
                            (LocalVariables|SetCurrentReason -977))))))))))
          (:CastFailed
            (LocalVariables|SetCurrentReason -1)))))
    (:then_1
      (return (LocalVariables|GetCurrentReason)))))

(fn BPOverrideCantBuildReasonString
  (params (CantBuildReason :type Integer))
  (LocalVariables|SetReasonFailed "")
  (switch int CantBuildReason
    (:Default
      _)
    (:-979
      (LocalVariables|SetReasonFailed "Too Much Rotation"))
    (:-978
      (LocalVariables|SetReasonFailed "Obstructed"))
    (:-977
      (LocalVariables|SetReasonFailed "Too High From Standing Location"))
    (:-976
      (LocalVariables|SetReasonFailed "Obstructed"))
    (:-975
      (LocalVariables|SetReasonFailed "Too Close To Ground"))
    (:-974
      (LocalVariables|SetReasonFailed "Object In Standing Location")))
  (return (LocalVariables|GetReasonFailed)))

(fn BPCanFinalPlaceonStructureSaddle
  (params (data :type Placement%20Data%20Structure%20%28by%20ref%29) (AttachToPawn :type Pawn%20Object%20Reference))
  (bind _parentstructure (Utilities|Struct|BreakPlacementData data))
  (bind _saddledino (Variables|/Script/ShooterGame.PrimalStructure|GetSaddleDino _parentstructure))
  (LocalVariables|SetreturnIsValid false)
  (Utilities|FlowControl|Sequence
    (:then_0
      (if (Math|Boolean|ANDBoolean (Utilities|IsValid _parentstructure) (Utilities|IsValid AttachToPawn) (Utilities|IsValid _saddledino) (== _saddledino AttachToPawn))
        (LocalVariables|SetreturnIsValid true)))
    (:then_1
      (return (LocalVariables|GetreturnIsValid)))))

(fn BPAllowSeating
  (params (ForController :type Controller%20Object%20Reference))
  (LocalVariables|SetbRetval true)
  (Utilities|FlowControl|Sequence
    (:then_0
      (if (not (Variables|Default|GetbSnappedIgnoreGroundForStandingLocation))
        (bind (_loc _rot _hitsomething) (CallFunction|GetStandingLocationRotation (Variables|Default|GetTraceType)))
        (bind (_loc_2 _rot_2 _hitsomething_2) (CallFunction|GetStandingLocationRotation "TraceTypeQuery4"))
        (LocalVariables|SetbRetval (Math|Boolean|ANDBoolean (<= (Math|Vector|VectorLength (- _loc _loc_2)) 1.0) _hitsomething_2 _hitsomething))))
    (:then_1
      (return (LocalVariables|GetbRetval)))))

(fn BPGetCameraLocationandRotation
  (params (InLocation :type Vector :default "0, 0, 0") (InRotation :type Rotator :default "0, 0, 0"))
  (bind _returnvalue (Transformation|GetActorForwardVector))
  (bind _cameraoffset (Variables|Default|GetCameraOffset))
  (bind (_x _y _z) (Math|Vector|BreakVector _cameraoffset))
  (return (+ (Transformation|GetActorLocation) (* _returnvalue _x) (* (Transformation|GetActorUpVector) _z)) (select (Variables|Default|GetUseFixedYaw) (Math|Conversions|RotationFromXVector _returnvalue) InRotation)))

(fn GetStandingLocationRotation
  (params (Channel :type ETraceTypeQuery%20Enum :default "TraceTypeQuery1"))
  (bind _returnvalue (Transformation|GetActorForwardVector))
  (bind _returnvalue_2 (Transformation|GetActorRightVector))
  (bind _returnvalue_3 (Transformation|GetActorUpVector))
  (bind _returnvalue_4 (Transformation|GetActorLocation))
  (bind _rideroffset (Variables|Default|GetRiderOffset))
  (bind _seatedcharacter (Variables|Default|GetSeatedCharacter))
  (bind _returnvalue_5 (* _returnvalue _rideroffset))
  (bind _returnvalue_6 (+ _returnvalue_4 _returnvalue_5))
  (LocalVariables|SetzHalfHeightOffset 0.0)
  (Utilities|IsValid _seatedcharacter
    (:Is%20Valid
      (LocalVariables|SetzHalfHeightOffset (Variables|/Script/Engine.CapsuleComponent|GetCapsuleHalfHeight (Variables|/Script/Engine.Character|GetCapsuleComponent _seatedcharacter))))
    (:Is%20Not%20Valid
      (bind _returnvalue_7 (Class|VictoryCore|GetClassDefaultObject "/Script/ShooterGame.ShooterCharacter"))
      (bind _asshootercharacter (Utilities|Casting|CastToShooterCharacter _returnvalue_7)
        (:then
          (LocalVariables|SetzHalfHeightOffset (Variables|/Script/Engine.CapsuleComponent|GetCapsuleHalfHeight (Variables|/Script/Engine.Character|GetCapsuleComponent _asshootercharacter))))
        (:CastFailed
          _))))
  (bind (_outhit _returnvalue_8) (Class|KismetSystemLibrary|SphereTraceSingleNEW (+ _returnvalue_6 (* _returnvalue_3 3e+01)) (+ (* (* _returnvalue_3 -1.0) (* (Variables|Default|GetLookForGroundDistance) 1.2)) _returnvalue_6) 2e+01 Channel false (Utilities|Array|MakeArray (Variables|Default|GetSeatedCharacter)) "None" true))
  (return (Math|Vector|SelectVector (+ (.ImpactPoint (Collision|BreakHitResult _outhit)) (Math|Vector|MakeVector 0.0 0.0 (LocalVariables|GetzHalfHeightOffset))) _returnvalue_6 _returnvalue_8) (Math|Rotator|SelectRotator (Class|KismetMathLibrary|MakeRot (.Pitch (Class|KismetMathLibrary|BreakRot (Math|Rotator|MakeRotationfromAxes (Math|Vector|ProjectVectorontoPlane _returnvalue (Transformation|GetActorUpVector (.HitActor (Collision|BreakHitResult _outhit)))) (Math|Vector|ProjectVectorontoPlane _returnvalue_2 (Transformation|GetActorUpVector (.HitActor (Collision|BreakHitResult _outhit)))) (Transformation|GetActorUpVector (.HitActor (Collision|BreakHitResult _outhit)))))) (.Yaw (Class|KismetMathLibrary|BreakRot (Math|Rotator|MakeRotationfromAxes (Math|Vector|ProjectVectorontoPlane _returnvalue (Transformation|GetActorUpVector (.HitActor (Collision|BreakHitResult _outhit)))) (Math|Vector|ProjectVectorontoPlane _returnvalue_2 (Transformation|GetActorUpVector (.HitActor (Collision|BreakHitResult _outhit)))) (Transformation|GetActorUpVector (.HitActor (Collision|BreakHitResult _outhit)))))) (.Roll (Class|KismetMathLibrary|BreakRot (Math|Rotator|MakeRotationfromAxes (Math|Vector|ProjectVectorontoPlane _returnvalue (Transformation|GetActorUpVector (.HitActor (Collision|BreakHitResult _outhit)))) (Math|Vector|ProjectVectorontoPlane _returnvalue_2 (Transformation|GetActorUpVector (.HitActor (Collision|BreakHitResult _outhit)))) (Transformation|GetActorUpVector (.HitActor (Collision|BreakHitResult _outhit))))))) (Class|KismetMathLibrary|MakeRot 0.0 (.Yaw (Class|KismetMathLibrary|BreakRot (Math|Rotator|MakeRotationfromAxes _returnvalue _returnvalue_2 _returnvalue_3))) 0.0) _returnvalue_8) _returnvalue_8))

(fn BPOverridePlacementLocation
  (params (PlacementLocation :type Vector :default "0, 0, 0"))
  (LocalVariables|SetNewLocation PlacementLocation)
  (Utilities|FlowControl|Sequence
    (:then_0
      (bind (_outhit _returnvalue) (Class|KismetSystemLibrary|SphereTraceSingleNEW (+ PlacementLocation "0, 0,50.000000") (- PlacementLocation "0, 0,10.000000") 2e+01 (Variables|Default|GetTraceType) false 0 "None" true))
      (if _returnvalue
        (LocalVariables|SetNewLocation (.ImpactPoint (Collision|BreakHitResult _outhit)))))
    (:then_1
      (return (LocalVariables|GetNewLocation)))))

(fn OnStartFire
  (|CallParentFunction)
  (bind _returnvalue (Class|PrimalStructureTurretBallista|GetCurrentAmmoType))
  (bind _returnvalue_2 (Class|PrimalStructureTurretBallista|CanFire))
  (if (and _returnvalue_2 (== _returnvalue (Variables|Default|Getgreek%20fire%20class)))
    (Class|Actor|ActorPlaySound (Variables|Default|Getgreek%20fire%20start%20sound) true "None" "0, 0, 0")))

(fn LookforStandingLocation
  (bind _seatedcharacter (Variables|Default|GetSeatedCharacter))
  (if (not (Networking|IsDedicatedServer))
    (Utilities|IsValid _seatedcharacter
      (:Is%20Valid
        (bind (_location _rotation) (CallFunction|GetFixedRiderLocation))
        (Transformation|SetActorLocationAndRotation _seatedcharacter _location _rotation)))))

(fn IsLocCloseEnough
  (params (Loc :type Vector))
  (LocalVariables|SetreturnValid false)
  (Utilities|FlowControl|Sequence
    (:then_0
      (LocalVariables|SetreturnValid (<= (Math|Vector|VectorLength (- Loc (+ (+ (Transformation|GetActorLocation) (Math|Vector|RotateVector (Math|Vector|MakeVector 0.0 0.0 4e+01) (Transformation|GetActorRotation))) (* (Transformation|GetActorForwardVector) (Variables|Default|GetRiderOffset))))) (* (Variables|Default|GetLookForGroundDistance) 0.5))))
    (:then_1
      (return (LocalVariables|GetreturnValid)))))